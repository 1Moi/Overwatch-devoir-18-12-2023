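; BP_Sticky is a timed area-knockback actor in Tracer's folder, apparently a sticky bomb, with no damage or sticking logic of its own.
; Two seconds after BeginPlay it draws a debug sphere and branches on the overlap result before that query has run.
; The false branch sphere-overlaps nearby pawns and launches OverwatchBaseCharacters radially outward by ForceAoe.
; DestroyActor sits inside the loop after each launch, or on the true branch.
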(event `self.ReceiveBeginPlay`
  (bind _returnvalue (`self.K2_GetActorLocation`))
  (`KismetSystemLibrary.Delay` 2.0)
  (`KismetSystemLibrary.DrawDebugSphere` _returnvalue 200.0 12 (struct :`R` 1.0 :`G` 1.0 :`B` 1.0 :`A` 1.0) 3.0)
  (if (stale _returnvalue_2)
    (`self.K2_DestroyActor`)
    (else
      (bind (_outactors _returnvalue_2) (`KismetSystemLibrary.SphereOverlapActors` _returnvalue 200.0 (`|MakeArray` "ObjectTypeQuery3" :!type "EObjectTypeQuery Enum")))
      (for _array_element _outactors
        (`KismetSystemLibrary.PrintString` (`KismetSystemLibrary.GetDisplayName` _array_element))
        (bind _asoverwatch_base_character (cast `/Game/OverwatchCharacters/OverwatchBaseCharacter` _array_element))
        (`Character.LaunchCharacter` _asoverwatch_base_character (* (`KismetMathLibrary.Normal` (- (`self.K2_GetActorLocation` _array_element) (`self.K2_GetActorLocation`))) (`self.Force Aoe`)) true true)
        (`self.K2_DestroyActor`)))))

(event `self.ReceiveTick`
  (params (DeltaSeconds :type "Float (single-precision)")))

(fn `UserConstructionScript`)