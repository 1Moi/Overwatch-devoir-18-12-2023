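; Spider bomb actor for the Fatale character that acts as a proximity knockback trap, with no damage logic.
; Every Tick it runs a fixed-radius sphere overlap for pawns, printing the name of each hit.
; Any OverwatchBaseCharacter found is launched directly away from the bomb, scaled by ForceAoe, and the bomb destroys itself.
; BeginPlay draws a long-lived debug sphere showing the trigger radius.
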(event `self.ReceiveBeginPlay`
  (`KismetSystemLibrary.DrawDebugSphere` (`self.K2_GetActorLocation`) 200.0 12 (struct :`R` 0.934923 :`G` 1.0 :`A` 1.0) 99999.0 1.0))

(event `self.ReceiveTick`
  (params (DeltaSeconds :type "Float (single-precision)"))
  (bind _outactors (`KismetSystemLibrary.SphereOverlapActors` (`self.K2_GetActorLocation`) 200.0 (`|MakeArray` "ObjectTypeQuery3" :!type "EObjectTypeQuery Enum")))
  (for _array_element _outactors
    (`KismetSystemLibrary.PrintString` (`KismetSystemLibrary.GetDisplayName` _array_element))
    (bind _asoverwatch_base_character (cast `/Game/OverwatchCharacters/OverwatchBaseCharacter` _array_element))
    (`Character.LaunchCharacter` _asoverwatch_base_character (* (`KismetMathLibrary.Normal` (- (`self.K2_GetActorLocation` _array_element) (`self.K2_GetActorLocation`))) (`self.Force Aoe`)) true true)
    (`self.K2_DestroyActor`)))

(fn `UserConstructionScript`)